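; StatisticGI is a Game Instance Blueprint for a pong game that keeps player statistics and persists them between sessions.
; On Init it runs LoadGame, which copies Statistics from the PongSaveGame in the PingPongSlot save slot when one exists.
; SaveGame reuses the existing save object or creates a new one, then writes the current Statistics back to that slot.
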(event `Save Game`
  (bind _returnvalue (`GameplayStatics.DoesSaveGameExist` "PingPongSlot"))
  (if _returnvalue
    (bind _returnvalue_2 (`GameplayStatics.LoadGameFromSlot` "PingPongSlot"))
    (bind _aspong_save_game (cast `/Game/Blueprints/PongSaveGame` _returnvalue_2))
    (set `self.Save` _aspong_save_game)
    (else
      (bind _returnvalue_3 (`GameplayStatics.CreateSaveGameObject` "/Game/Blueprints/PongSaveGame.PongSaveGame_C"))
      (set `self.Save` _returnvalue_3)))
  (set `/Game/Blueprints/PongSaveGame.Statistics` (`self.Statistics`) (`self.Save`))
  (`GameplayStatics.SaveGameToSlot` (`self.Save`) "PingPongSlot"))

(event `Load Game`
  (bind _returnvalue (`GameplayStatics.DoesSaveGameExist` "PingPongSlot"))
  (if _returnvalue
    (bind _returnvalue_2 (`GameplayStatics.LoadGameFromSlot` "PingPongSlot"))
    (bind _aspong_save_game (cast `/Game/Blueprints/PongSaveGame` _returnvalue_2))
    (bind _output_get (set `self.Save` _aspong_save_game))
    (set `self.Statistics` (`/Game/Blueprints/PongSaveGame.Statistics` _output_get))))

(event `self.ReceiveInit`
  (`self.Load Game`))